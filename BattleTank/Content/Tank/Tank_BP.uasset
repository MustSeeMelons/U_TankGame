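; Player-controllable tank Blueprint that handles camera aim input and firing.
; On BeginPlay it hands its Barrel and Turret components to setter functions that are not defined in this graph.
; Azimuth and elevation axes rotate a two-part camera gimbal, yawing AzimuthGimbal and pitching SpringArm separately, scaled by delta time.
; The Fire action calls Fire, also defined outside this graph; the construction script is empty.
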(event `self.ReceiveBeginPlay`
  (`self.SetBarrelReferrence` (`self.Barrel`))
  (`self.SetTurretReferrence` (`self.Turret`)))

(event `InputAxis|AizAzimuth`
  (params (AxisValue :type "Float (single-precision)"))
  ;[1 1 1] Input binding
  (`SceneComponent.K2_AddLocalRotation` (`self.AzimuthGimbal`) (`KismetMathLibrary.MakeRotator` 0.0 0.0 (* AxisValue (`GameplayStatics.GetWorldDeltaSeconds`) 100.0)) false false))

(event `InputAxis|AimElavation`
  (params (AxisValue :type "Float (single-precision)"))
  ;[1 1 1] Input binding
  (`SceneComponent.K2_AddLocalRotation` (`self.SpringArm`) (`KismetMathLibrary.MakeRotator` 0.0 (* AxisValue (`GameplayStatics.GetWorldDeltaSeconds`) 100.0)) false false))

(event `InputAction|Fire`
  (params (Key :type "Key Structure"))
  ;[1 1 1] Input binding
  (:`Pressed`
    (`self.Fire`)))

(fn `UserConstructionScript`)